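; BP_Wolf is a wolf actor that makes a one-time creep toward a deer.
; SetCreeping starts the creep only once, guarded by HasCrept.
; While IsCreeping is set, Tick moves the wolf along world +Y at MoveSpeed scaled by delta time, without tracking the deer's position.
; Overlapping a BP_Deer clears IsCreeping and stops the movement.
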(event EventBeginPlay)

(event Collision|EventActorBeginOverlap
  (params (OtherActor :type Actor%20Object%20Reference))
  (Utilities|Casting|CastToBP_Deer OtherActor)
  (Variables|Default|SetIsCreeping false))

(event EventTick
  (params (DeltaSeconds :type Float%20%28single-precision%29))
  (if (Variables|Default|GetIsCreeping)
    (CallFunction|CreepTowardsDeer DeltaSeconds)))

(fn ConstructionScript)

(fn CreepTowardsDeer
  (params (deltaSeconds :type Float%20%28double-precision%29))
  (bind _returnvalue (Transformation|GetActorLocation))
  (Transformation|SetActorLocation (Math|Vector|MakeVector (.x _returnvalue) (+ (.y _returnvalue) (* (Variables|Default|GetMoveSpeed) deltaSeconds)) (.z _returnvalue)) false false))

(fn SetCreeping
  (if (not (Variables|Default|GetHasCrept))
    (Variables|Default|SetIsCreeping true)
    (Variables|Default|SetHasCrept true)))