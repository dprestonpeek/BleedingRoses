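; BP_Deer is a deer actor that topples over when a BP_Wolf overlaps it.
; The overlap event casts the other actor to BP_Wolf and calls Die, which rolls the root component 90 degrees onto its side with no effective change in location.
; Die is gated by IsDead but never sets that flag here.
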(event EventBeginPlay)

(event Collision|EventActorBeginOverlap
  (params (OtherActor :type Actor%20Object%20Reference))
  (Utilities|Casting|CastToBP_Wolf OtherActor)
  (CallFunction|Die))

(event EventTick
  (params (DeltaSeconds :type Float%20%28single-precision%29)))

(fn ConstructionScript)

(fn Die
  (bind _defaultsceneroot (Variables|Default|GetDefaultSceneRoot))
  (bind _relativelocation (Variables|/Script/Engine.SceneComponent|GetRelativeLocation _defaultsceneroot))
  (bind _relativerotation (Variables|/Script/Engine.SceneComponent|GetRelativeRotation _defaultsceneroot))
  (if (not (Variables|Default|GetIsDead))
    (Transformation|SetRelativeLocationAndRotation _defaultsceneroot (Math|Vector|MakeVector (.x _relativelocation) (.y _relativelocation) (- (.z _relativelocation) 0.0)) (Math|Rotator|MakeRotator (+ (.roll _relativerotation) 9e+01) (.pitch _relativerotation) (.yaw _relativerotation)) false false)))